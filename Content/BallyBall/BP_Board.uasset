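; BP_Board is the brick board for BallyBall, an actor that spawns and clears the field of BP_Brick actors.
; SpawnBricks uses nested loops and range mapping to lay out a five-by-five grid centered on the board, with world-axis offsets and the board's rotation on each brick.
; Clear destroys every BP_Brick in the world, not just its own.
; BeginPlay is empty, so neither event runs automatically.
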(event Custom|SpawnBricks
  (for _index (range 1 5)
    (for _index_2 (range 1 5)
      (Game|SpawnActorfromClass "/Game/BallyBall/BP_Brick.BP_Brick_C" (Math|Transform|MakeTransform (+ (Math|Vector|MakeVector (Math|Float|MapRangeClamped (Math|Conversions|ToFloat(Integer) _index_2) 1.0 5.0 -1e+02 1e+02) (Math|Float|MapRangeClamped (Math|Conversions|ToFloat(Integer) _index) 1.0 5.0 -3e+02 3e+02) 0.0) (Transformation|GetActorLocation)) (Transformation|GetActorRotation) "1,1,1") "Undefined" 0 0))))

(event Custom|Clear
  (bind _outactors (Actor|GetAllActorsOfClass "/Game/BallyBall/BP_Brick.BP_Brick_C"))
  (for _array_element _outactors
    (Actor|DestroyActor _array_element)))

(event EventBeginPlay)

(fn ConstructionScript)