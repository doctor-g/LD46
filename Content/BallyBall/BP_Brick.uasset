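; BP_Brick is a destructible brick in BallyBall that breaks on any damage.
; The construction script picks a random material from the Colors array, and BeginPlay turns it into a dynamic material instance.
; On damage it fires the OnBrickDestroyed dispatcher, spawns an explosion particle effect and disables mesh collision.
; A FadeOut timeline then drives the material's opacity and emissive intensity before destroying the actor.
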(event EventBeginPlay
  (bind _staticmesh (Variables|Default|GetStaticMesh))
  ;[1 1 1] BeginPlay: Set up dynamic material instance
  (bind _returnvalue (Rendering|Material|CreateDynamicMaterialInstance _staticmesh 0 (Rendering|Material|GetMaterial _staticmesh 0) "None" :!class /Script/Engine.PrimitiveComponent))
  (Variables|Default|SetDynamicMaterial _returnvalue))

(event Game|Damage|EventAnyDamage
  (params (Damage :type Float%20%28single-precision%29) (DamageType :type Damage%20Type%20Object%20Reference) (InstigatedBy :type Controller%20Object%20Reference) (DamageCauser :type Actor%20Object%20Reference))
  (bind _dynamicmaterial (Variables|Default|GetDynamicMaterial))
  (Default|CallOnBrickDestroyed)
  (Effects|SpawnEmitteratLocation "/Game/BallyBall/PS_BlockExplosion.PS_BlockExplosion" (Transformation|GetActorLocation))
  (Collision|SetCollisionEnabled (Variables|Default|GetStaticMesh) "NoCollision")
  (bind (_direction _opacity _emissiveintensity) (Timeline|FadeOut PlayFromStart)
    (:Update
      (Rendering|Material|SetScalarParameterValue _dynamicmaterial "Opacity" _opacity :!class /Script/Engine.MaterialInstanceDynamic)
      (Rendering|Material|SetScalarParameterValue _dynamicmaterial "EmissiveIntensity" _emissiveintensity :!class /Script/Engine.MaterialInstanceDynamic))
    (:Finished
      (Actor|DestroyActor))))

(fn ConstructionScript
  (bind _colors (LocalVariables|GetColors))
  (Rendering|Material|SetMaterial (Variables|Default|GetStaticMesh) 0 (Utilities|Array|Get(acopy) _colors (Math|Random|RandomIntegerinRange 0 (- (Utilities|Array|Length _colors) 1)))))