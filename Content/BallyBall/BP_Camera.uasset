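; Camera Blueprint for BallyBall that drives a fisheye lens post-process effect reacting to ball hits.
; On BeginPlay it installs a dynamic lens material as a post-process blendable and subscribes to the game mode's ball spawn event.
; Ball hits boost the intensity component's target intensity.
; Each tick it feeds the current intensity and the ball's normalized screen position to the material, centering the distortion on the ball.
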(event Custom|OnBallSpawn
  (params (Ball :type BP%20Ball%20Object%20Reference))
  ;[1 1 1] When anything is hit by the ball, increase the intensity of the lens effect
  (Variables|Default|SetBall Ball)
  (Collision|BindEventtoOnComponentHit (Variables|/Script/BallyBall.Ball|GetMeshComponent Ball) (delegate Custom|OnBallHitSomething)))

(event Custom|OnBallHitSomething
  (params (HitComponent :type Primitive%20Component%20Object%20Reference) (OtherActor :type Actor%20Object%20Reference) (OtherComp :type Primitive%20Component%20Object%20Reference) (NormalImpulse :type Vector) (Hit :type Hit%20Result%20Structure%20%28by%20ref%29))
  ;[1 1 1] When anything is hit by the ball, increase the intensity of the lens effect
  (Class|FloatInterpFalloffComponent|BoostTargetIntensity (Variables|Default|GetIntensityComponent) (Variables|Default|GetIntensityGainPerHit)))

(event EventBeginPlay
  ;[1 1 1] When anything is hit by the ball, increase the intensity of the lens effect
  (bind _asbp_game_mode (Utilities|Casting|CastToBP_GameMode (Game|GetGameMode)))
  (EventDispatchers|BindEventtoOnBallSpawn _asbp_game_mode (delegate Custom|OnBallSpawn))
  ;[1 1 1] Set up lens effect as dynamic material instance
  (bind _returnvalue (Rendering|Material|CreateDynamicMaterialInstance "/Game/BallyBall/MI_LensEffect.MI_LensEffect" "None" :!class /Script/Engine.KismetMaterialLibrary))
  (Variables|Default|SetLensEffectMaterial _returnvalue)
  (Variables|/Script/Engine.PostProcessComponent|SetSettings (Variables|Default|GetPostProcess) (Utilities|Struct|MakePostProcessSettings (Utilities|Struct|MakeWeightedBlendables (Utilities|Array|MakeArray (Utilities|Struct|MakeWeightedBlendable 1.0 _returnvalue))))))

(event EventTick
  (params (DeltaSeconds :type Float%20%28single-precision%29))
  (bind _lenseffectmaterial (Variables|Default|GetLensEffectMaterial))
  ;[1 1 1] Update the lens effect
  (Rendering|Material|SetScalarParameterValue _lenseffectmaterial "Intensity" (Variables|/Script/BallyBall.FloatInterpFalloffComponent|GetIntensity (Variables|Default|GetIntensityComponent)) :!class /Script/Engine.MaterialInstanceDynamic)
  ;[1 1 1] Focus the fisheye on the ball position, if we have a valid ball reference
  (bind _ball (Variables|Default|GetBall)
    (:then
      (Rendering|Material|SetVectorParameterValue _lenseffectmaterial "BallPositionSS" (Math|Conversions|ToLinearColor(Vector) (Math|Vector|MakeVector (.x (/ (.ScreenPosition (Class|GameplayStatics|ProjectWorldtoScreen (Game|GetPlayerController 0) (Transformation|GetWorldLocation (Variables|/Script/BallyBall.Ball|GetMeshComponent _ball)) false)) (Viewport|GetViewportSize))) (.y (/ (.ScreenPosition (Class|GameplayStatics|ProjectWorldtoScreen (Game|GetPlayerController 0) (Transformation|GetWorldLocation (Variables|/Script/BallyBall.Ball|GetMeshComponent _ball)) false)) (Viewport|GetViewportSize))) 0.0)) :!class /Script/Engine.MaterialInstanceDynamic))
    (:else)))

(fn ConstructionScript)