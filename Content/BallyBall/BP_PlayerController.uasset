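; Player controller for BallyBall, a paddle-and-brick game, that drives the title, game and end flow through a State variable.
; Launch starts the game and spawns bricks, requests a ball from the paddle when the game mode allows, or clears boards returning to title.
; ChangeCamera blends to tagged cameras, holding transitional states that ignore Launch until the blend ends.
; Game over triggers the end camera; other inputs kill all bricks mid-game or quit.
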(event Custom|OnGameOver
  (Utilities|ChangeCamera "EndCamera" "NewEnumerator3" "NewEnumerator4"))

(event EventBeginPlay
  (bind _asbp_game_mode (Utilities|Casting|CastToBP_GameMode (Game|GetGameMode)))
  (EventDispatchers|BindEventtoOnGameOver _asbp_game_mode (delegate Custom|OnGameOver)))

(event Input|ActionEvents|InputActionLaunch
  (params (Key :type Key%20Structure :default "None"))
  (:Pressed
    (switch Utilities|FlowControl|Switch|SwitchonEPlayerControllerState (Variables|Default|GetState)
      (:NewEnumerator0
        ;[1 1 1] Start playing
        (Default|StartGame (.AsBP%20Game%20Mode (Utilities|Casting|CastToBP_GameMode (Game|GetGameMode))))
        (Audio|PlaySound2D "/Game/BallyBall/Audio/A_PaddleBounce.A_PaddleBounce" 1.0 1.0 0.0 0 0)
        (bind _outactors (Actor|GetAllActorsOfClass "/Game/BallyBall/BP_Board.BP_Board_C"))
        (for _array_element _outactors
          (Default|SpawnBricks _array_element))
        (Utilities|ChangeCamera "GameCamera" "NewEnumerator1" "NewEnumerator2"))
      (:NewEnumerator2
        ;[1 1 1] Spawn a ball if we can
        (bind _asbp_game_mode (Utilities|Casting|CastToBP_GameMode (Game|GetGameMode)))
        (bind _canspawn (Default|CanSpawnBall _asbp_game_mode))
        (if _canspawn
          (bind _asbp_paddle (Utilities|Casting|CastToBP_Paddle (Pawn|GetControlledPawn)))
          (bind _ball (Default|SpawnBall _asbp_paddle))
          (bind _asbp_game_mode_2 (Utilities|Casting|CastToBP_GameMode (Game|GetGameMode)))
          (Default|CallOnBallSpawn _asbp_game_mode_2 _ball)))
      (:NewEnumerator4
        (Audio|PlaySound2D "/Game/BallyBall/Audio/A_PaddleBounce.A_PaddleBounce" 1.0 1.0 0.0 0 0)
        (Utilities|ChangeCamera "TitleCamera" "NewEnumerator5" "NewEnumerator0")
        (bind _outactors_2 (Actor|GetAllActorsOfClass "/Game/BallyBall/BP_Board.BP_Board_C"))
        (for _array_element_2 _outactors_2
          (Default|Clear _array_element_2))))))

(event Input|ActionEvents|InputActionKillAllBlocks
  (params (Key :type Key%20Structure :default "None"))
  (:Pressed
    (switch Utilities|FlowControl|Switch|SwitchonEPlayerControllerState (Variables|Default|GetState)
      (:NewEnumerator2
        (bind _outactors (Actor|GetAllActorsOfClass "/Game/BallyBall/BP_Brick.BP_Brick_C"))
        (for _array_element _outactors
          (Default|Kill _array_element))))))

(event Input|ActionEvents|InputActionQuit
  (params (Key :type Key%20Structure :default "None"))
  (:Pressed
    (Game|QuitGame self "Quit" false)))

(fn ConstructionScript)

(fn FindCamerabyTag
  (params (ActorTag :type Name))
  (bind _outactors (Actor|GetAllActorswithTag ActorTag))
  (bind _ascamera_actor (Utilities|Casting|CastToCameraActor (Utilities|Array|Get(acopy) _outactors)))
  (return _ascamera_actor))