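; BP_Ball is the ball actor in BallyBall, glowing with an intensity that rises on impacts.
; It creates a dynamic material at BeginPlay, boosts its IntensityComponent on each hit, and copies that intensity to the material's glow every tick.
; Kill fires a ball-killed notification, plays a lose sound, animates opacity through a timeline, then destroys the actor.
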(event Custom|Kill
  (Default|CallOnBallKilled)
  (Audio|PlaySound2D "/Game/BallyBall/Audio/A_LoseBall.A_LoseBall" 1.0 1.0 0.0 0 0)
  (bind _opacity (Timeline|Timeline_0 PlayFromStart)
    (:Update
      (Rendering|Material|SetScalarParameterValue (Variables|Default|GetDynamicMaterial) "Opacity" _opacity :!class /Script/Engine.MaterialInstanceDynamic))
    (:Finished
      (Actor|DestroyActor))))

(event EventBeginPlay
  ;[1 1 1] BeginPlay: Initialize dynamic material instance
  (bind _returnvalue (Rendering|Material|CreateDynamicMaterialInstance (Variables|Default|GetMeshComponent) 0 "/Game/BallyBall/M_Ball.M_Ball" "None" :!class /Script/Engine.PrimitiveComponent))
  (Variables|Default|SetDynamicMaterial _returnvalue))

(event Collision|EventHit
  (params (MyComp :type Primitive%20Component%20Object%20Reference) (Other :type Actor%20Object%20Reference) (OtherComp :type Primitive%20Component%20Object%20Reference) (bSelfMoved :type Boolean) (HitLocation :type Vector :default "0, 0, 0") (HitNormal :type Vector :default "0, 0, 0") (NormalImpulse :type Vector :default "0, 0, 0") (Hit :type Hit%20Result%20Structure%20%28by%20ref%29))
  ;[1 1 1] When hitting something, boost intensity
  (Class|FloatInterpFalloffComponent|BoostTargetIntensity (Variables|Default|GetIntensityComponent) 0.5))

(event EventTick
  (params (DeltaSeconds :type Float%20%28single-precision%29))
  ;[1 1 1] Update the intensity of the Ball
  (Rendering|Material|SetScalarParameterValue (Variables|Default|GetDynamicMaterial) "GlowIntensity" (Variables|/Script/BallyBall.FloatInterpFalloffComponent|GetIntensity (Variables|Default|GetIntensityComponent)) :!class /Script/Engine.MaterialInstanceDynamic))

(fn ConstructionScript)