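; BP_Rails is a rail actor that animates its emissive glow when something hits it.
; The construction script creates one dynamic instance of M_Pipe and assigns it to the first material slot of every static mesh component.
; BeginPlay binds each mesh's hit event to a handler that restarts a timeline driving the EmissiveIntensity parameter.
; Because the meshes share that instance, a hit on any piece animates all of them together.
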(event Custom|OnRailsHit
  (params (HitComponent :type Primitive%20Component%20Object%20Reference) (OtherActor :type Actor%20Object%20Reference) (OtherComp :type Primitive%20Component%20Object%20Reference) (NormalImpulse :type Vector) (Hit :type Hit%20Result%20Structure%20%28by%20ref%29))
  (bind _alpha (Timeline|Timeline_0 PlayFromStart)
    (:Update
      (Rendering|Material|SetScalarParameterValue (Variables|Default|GetDynamicMaterial) "EmissiveIntensity" _alpha :!class /Script/Engine.MaterialInstanceDynamic))))

(event EventBeginPlay
  (for _array_element (Actor|GetComponentsByClass "/Script/Engine.StaticMeshComponent")
    (Collision|BindEventtoOnComponentHit _array_element (delegate Custom|OnRailsHit))))

(event EventTick
  (params (DeltaSeconds :type Float%20%28single-precision%29)))

(fn ConstructionScript
  (bind _returnvalue (Rendering|Material|CreateDynamicMaterialInstance "/Game/BallyBall/M_Pipe.M_Pipe" "None" :!class /Script/Engine.KismetMaterialLibrary))
  (Variables|Default|SetDynamicMaterial _returnvalue)
  (for _array_element (Actor|GetComponentsByClass "/Script/Engine.StaticMeshComponent")
    (Rendering|Material|SetMaterial _array_element 0 (Variables|Default|GetDynamicMaterial))))